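; Boss keycard pickup that stays hidden and non-collidable until the game instance reports the boss dead.
; Tick polls that flag, then shows the paper sprite, enables the box collision and yaws the actor toward the player as a billboard.
; The Keycard enum picks the red, orange or blue sprite at construction.
; On player overlap it sets the matching character flag, updates the HUD and destroys itself.
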(event `self.ReceiveBeginPlay`
  (`SceneComponent.SetVisibility` (`self.PaperSprite`) false false)
  (`PrimitiveComponent.SetCollisionEnabled` (`self.Box`) "NoCollision"))

(event `self.ReceiveTick`
  (params (DeltaSeconds :type "Float (single-precision)"))
  (bind (_returnvalue_roll _returnvalue_pitch _returnvalue_yaw) (`KismetMathLibrary.BreakRotator` (`KismetMathLibrary.FindLookAtRotation` (`self.K2_GetActorLocation`) (`self.K2_GetActorLocation` (`GameplayStatics.GetPlayerCharacter` 0)))))
  (bind _asboss_game_instance (cast `/Game/Enemies/BossGameInstance` (`GameplayStatics.GetGameInstance`)))
  (if (`/Game/Enemies/BossGameInstance.BossDead?` _asboss_game_instance)
    (`self.K2_SetActorRotation` (`KismetMathLibrary.MakeRotator` 0.0 0.0 _returnvalue_yaw))
    (`SceneComponent.SetVisibility` (`self.PaperSprite`) true false)
    (`PrimitiveComponent.SetCollisionEnabled` (`self.Box`) "QueryAndPhysics")))

(event `self.Box.OnComponentBeginOverlap`
  (params (OverlappedComponent :type "PrimitiveComponent Object Reference") (OtherActor :type "Actor Object Reference") (OtherComp :type "PrimitiveComponent Object Reference") (OtherBodyIndex :type Integer) (bFromSweep :type Boolean) (SweepResult :type "HitResult Structure (by ref)"))
  (bind _firstpersoncharacterreference (`self.FirstPersonCharacterReference`))
  (bind _firstpersoncharacterreference_2 (`self.FirstPersonCharacterReference`))
  (bind _firstpersoncharacterreference_3 (`self.FirstPersonCharacterReference`))
  (bind _asbp_first_person_character (cast `/Game/FirstPerson/Blueprints/BP_FirstPersonCharacter` OtherActor))
  (set `self.FirstPersonCharacterReference` _asbp_first_person_character)
  (switch `/Game/Blueprints/Items/Keycard` (`self.Keycard`)
    (:`NewEnumerator0`
      (set `/Game/FirstPerson/Blueprints/BP_FirstPersonCharacter.RedKeycard?` true _firstpersoncharacterreference_2)
      (`/Game/Blueprints/UI/PlayerHUD.FindRedKeycard` (`/Game/FirstPerson/Blueprints/BP_FirstPersonCharacter.PlayerHUD` _firstpersoncharacterreference_2))
      (`self.K2_DestroyActor`))
    (:`NewEnumerator1`
      (set `/Game/FirstPerson/Blueprints/BP_FirstPersonCharacter.OrangeKeycard?` true _firstpersoncharacterreference_3)
      (`/Game/Blueprints/UI/PlayerHUD.FindOrangeKeycard` (`/Game/FirstPerson/Blueprints/BP_FirstPersonCharacter.PlayerHUD` _firstpersoncharacterreference_3))
      (`self.K2_DestroyActor`))
    (:`NewEnumerator2`
      (set `/Game/FirstPerson/Blueprints/BP_FirstPersonCharacter.BlueKeycard?` true _firstpersoncharacterreference)
      (`/Game/Blueprints/UI/PlayerHUD.FindBlueKeycard` (`/Game/FirstPerson/Blueprints/BP_FirstPersonCharacter.PlayerHUD` _firstpersoncharacterreference))
      (`self.K2_DestroyActor`))))

(fn `UserConstructionScript`
  (switch `/Game/Blueprints/Items/Keycard` (`self.Keycard`)
    (:`NewEnumerator0`
      (`PaperSpriteComponent.SetSprite` (`self.PaperSprite`) "/Game/Sprites/Items/redkey_Sprite.redkey_Sprite"))
    (:`NewEnumerator1`
      (`PaperSpriteComponent.SetSprite` (`self.PaperSprite`) "/Game/Sprites/Items/orangekey_Sprite.orangekey_Sprite"))
    (:`NewEnumerator2`
      (`PaperSpriteComponent.SetSprite` (`self.PaperSprite`) "/Game/Sprites/Items/bluekey_Sprite.bluekey_Sprite"))))