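; A weapon pickup actor that gives the first-person character a weapon when they walk into it.
; The construction script maps the Weapon enum to a Paper2D sprite and the matching weapon class.
; Sphere overlap by the character calls PickupWeapon with that class and enum, then destroys the pickup.
; Each tick it yaws toward the player, billboarding the sprite.
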(event `self.Sphere.OnComponentBeginOverlap`
  (params (OverlappedComponent :type "PrimitiveComponent Object Reference") (OtherActor :type "Actor Object Reference") (OtherComp :type "PrimitiveComponent Object Reference") (OtherBodyIndex :type Integer) (bFromSweep :type Boolean) (SweepResult :type "HitResult Structure (by ref)"))
  (bind _asbp_first_person_character (cast `/Game/FirstPerson/Blueprints/BP_FirstPersonCharacter` OtherActor))
  (`/Game/FirstPerson/Blueprints/BP_FirstPersonCharacter.PickupWeapon` _asbp_first_person_character (`self.WeaponClass`) (`self.Weapon`))
  (`self.K2_DestroyActor`))

(event `self.ReceiveTick`
  (params (DeltaSeconds :type "Float (single-precision)"))
  (bind (_returnvalue_roll _returnvalue_pitch _returnvalue_yaw) (`KismetMathLibrary.BreakRotator` (`KismetMathLibrary.FindLookAtRotation` (`self.K2_GetActorLocation`) (`self.K2_GetActorLocation` (`GameplayStatics.GetPlayerCharacter` 0)))))
  (`self.K2_SetActorRotation` (`KismetMathLibrary.MakeRotator` 0.0 0.0 _returnvalue_yaw)))

(fn `UserConstructionScript`
  (switch `/Game/Blueprints/Weapons/Weapon` (`self.Weapon`)
    (:`NewEnumerator0`
      (`PaperSpriteComponent.SetSprite` (`self.PaperSprite`) "/Game/Sprites/Weapons/Shotgun/ShotgunSprite.ShotgunSprite")
      (set `self.WeaponClass` "/Game/Blueprints/Weapons/BP_Shotgun.BP_Shotgun_C"))
    (:`NewEnumerator1`
      (`PaperSpriteComponent.SetSprite` (`self.PaperSprite`) "/Game/Sprites/Weapons/MiniGun/MinigunSprite.MinigunSprite")
      (set `self.WeaponClass` "/Game/Blueprints/Weapons/BP_Minigun.BP_Minigun_C"))
    (:`NewEnumerator2`
      (`PaperSpriteComponent.SetSprite` (`self.PaperSprite`) "/Game/Sprites/Weapons/PlasmaGun/PlasmaSprite.PlasmaSprite")
      (set `self.WeaponClass` "/Game/Blueprints/Weapons/BP_PlasmaGun.BP_PlasmaGun_C"))
    (:`NewEnumerator3`
      (`PaperSpriteComponent.SetSprite` (`self.PaperSprite`) "/Game/Sprites/Weapons/RPG/RPGSprite.RPGSprite")
      (set `self.WeaponClass` "/Game/Blueprints/Weapons/BP_RPG.BP_RPG_C"))
    (:`NewEnumerator4`
      (`PaperSpriteComponent.SetSprite` (`self.PaperSprite`) "/Game/Sprites/Weapons/BFG/BFGSprite.BFGSprite")
      (set `self.WeaponClass` "/Game/Blueprints/Weapons/BP_BFG.BP_BFG_C"))
    (:`NewEnumerator5`
      (`PaperSpriteComponent.SetSprite` (`self.PaperSprite`) "/Game/Sprites/Weapons/Chainsaw/ChainsawSprite.ChainsawSprite")
      (set `self.WeaponClass` "/Game/Blueprints/Weapons/BP_Chainsaw.BP_Chainsaw_C"))))