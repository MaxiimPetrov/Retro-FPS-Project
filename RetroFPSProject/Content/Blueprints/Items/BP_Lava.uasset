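; BP_Lava is a lava hazard that damages the first-person player character while it stands inside the Box trigger.
; Box overlap starts a looping timer that repeatedly applies damage to the stored character, and end overlap clears that timer by its saved handle.
; Tick polls the BossGameInstance each frame and destroys the lava actor once BossDead is set.
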(event `self.ReceiveTick`
  (params (DeltaSeconds :type "Float (single-precision)"))
  (bind _asboss_game_instance (cast `/Game/Enemies/BossGameInstance` (`GameplayStatics.GetGameInstance`)))
  (if (`/Game/Enemies/BossGameInstance.BossDead?` _asboss_game_instance)
    (`self.K2_DestroyActor`)))

(event `self.Box.OnComponentBeginOverlap`
  (params (OverlappedComponent :type "PrimitiveComponent Object Reference") (OtherActor :type "Actor Object Reference") (OtherComp :type "PrimitiveComponent Object Reference") (OtherBodyIndex :type Integer) (bFromSweep :type Boolean) (SweepResult :type "HitResult Structure (by ref)"))
  (bind _asbp_first_person_character (cast `/Game/FirstPerson/Blueprints/BP_FirstPersonCharacter` OtherActor))
  (bind _returnvalue (`KismetSystemLibrary.K2_SetTimerDelegate` (delegate `LavaDamage`) 0.1 true))
  (set `self.LavaEvent` _returnvalue))

(event `LavaDamage`
  (`GameplayStatics.ApplyDamage` (stale `self.Box.OnComponentBeginOverlap` _asbp_first_person_character) 10.0))

(event `self.Box.OnComponentEndOverlap`
  (params (OverlappedComponent :type "PrimitiveComponent Object Reference") (OtherActor :type "Actor Object Reference") (OtherComp :type "PrimitiveComponent Object Reference") (OtherBodyIndex :type Integer))
  (cast `/Game/FirstPerson/Blueprints/BP_FirstPersonCharacter` OtherActor)
  (`KismetSystemLibrary.K2_ClearAndInvalidateTimerHandle` (`self.LavaEvent`)))

(fn `UserConstructionScript`)