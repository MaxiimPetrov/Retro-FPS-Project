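; Boss enemy Blueprint with a Paper2D flipbook that starts hidden and turns in yaw to face the player every tick.
; When PawnSensing sees a pawn, it reveals the flipbook, greatly extends its sight radius and flags the boss as activated in BossGameInstance.
; On destruction it flags the boss as dead there.
; Health is initialized on BeginPlay, but no damage handling lives in this graph.
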(event `self.ReceiveBeginPlay`
  (`SceneComponent.SetVisibility` (`self.PaperFlipbook`) false false)
  (set `self.Health` 100.0))

(event `self.ReceiveTick`
  (params (DeltaSeconds :type "Float (single-precision)"))
  (bind (_returnvalue_roll _returnvalue_pitch _returnvalue_yaw) (`KismetMathLibrary.BreakRotator` (`KismetMathLibrary.FindLookAtRotation` (`self.K2_GetActorLocation`) (`self.K2_GetActorLocation` (`GameplayStatics.GetPlayerCharacter` 0)))))
  (`self.K2_SetActorRotation` (`KismetMathLibrary.MakeRotator` 0.0 0.0 _returnvalue_yaw)))

(event `self.PawnSensing.OnSeePawn`
  (params (Pawn :type "Pawn Object Reference"))
  (bind _pawnsensing (`self.PawnSensing`))
  (set `PawnSensingComponent.SightRadius` (+ (`PawnSensingComponent.SightRadius` _pawnsensing) 30000.0) _pawnsensing)
  (`SceneComponent.SetVisibility` (`self.PaperFlipbook`) true false)
  (bind _asboss_game_instance (cast `/Game/Enemies/BossGameInstance` (`GameplayStatics.GetGameInstance`)))
  (set `/Game/Enemies/BossGameInstance.BossActivated` true _asboss_game_instance))

(event `self.ReceiveDestroyed`
  (bind _asboss_game_instance (cast `/Game/Enemies/BossGameInstance` (`GameplayStatics.GetGameInstance`)))
  (set `/Game/Enemies/BossGameInstance.BossDead?` true _asboss_game_instance))

(fn `UserConstructionScript`
  (`parent.UserConstructionScript`))